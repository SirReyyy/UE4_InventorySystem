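; Base container actor for the inventory system, with a lid, an inventory component and an overlap prompt.
; Interacting as a ThirdPersonCharacter plays a timeline that rotates the lid open and toggles the inventory; a separate close event reverses the animation.
; BeginPlay copies the Items array into the component's slots by index.
; A box trigger shows the inventory name as text during overlap and hides it afterwards.
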(event `OpenContainer`
  (bind (_direction _containerlid) (`Timeline|ContainerAnim` :!label _label)
    (:`Update`
      (`SceneComponent.K2_SetRelativeRotation` (`self.MeshTop`) (* (`self.LidRotation`) _containerlid) false false))))

(event `CloseContainer`
  (goto _label :!via `Reverse`))

(event `/Game/InventorySystem/Interfaces/Interact_Interface.Interact`
  (params (Interactor :type "Actor Object Reference"))
  (cast `/Game/ThirdPersonBP/Blueprints/ThirdPersonCharacter` Interactor)
  (`self.OpenContainer`)
  (`/Game/InventorySystem/Inventory_Component.F_ToggleInventory` (`self.Inventory_Component`)))

(event `self.ReceiveBeginPlay`
  (for (_array_element _array_index) (`self.Items`)
    (`KismetArrayLibrary.Array_Set` (`/Game/InventorySystem/Inventory_Component.InventorySlot` (`self.Inventory_Component`)) _array_index _array_element)))

(event `self.Box.OnComponentBeginOverlap`
  (params (OverlappedComponent :type "PrimitiveComponent Object Reference") (OtherActor :type "Actor Object Reference") (OtherComp :type "PrimitiveComponent Object Reference") (OtherBodyIndex :type Integer) (bFromSweep :type Boolean) (SweepResult :type "HitResult Structure (by ref)"))
  (bind _textrender (`self.TextRender`))
  (`SceneComponent.SetVisibility` _textrender true false)
  (`TextRenderComponent.K2_SetText` _textrender (`/Game/InventorySystem/Inventory_Component.InventoryName` (`self.Inventory_Component`))))

(event `self.Box.OnComponentEndOverlap`
  (params (OverlappedComponent :type "PrimitiveComponent Object Reference") (OtherActor :type "Actor Object Reference") (OtherComp :type "PrimitiveComponent Object Reference") (OtherBodyIndex :type Integer))
  (`SceneComponent.SetVisibility` (`self.TextRender`) false false))

(fn `UserConstructionScript`)